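; BP_BounceOrb is an orb actor that detonates when damaged and respawns after a short delay.
; On AnyDamage it prints the damage, plays a detonate flipbook, then hides itself and disables collision.
; It resets to the idle flipbook while hidden, then reappears with collision after a few seconds.
; Any bouncing behaviour is not in its graphs, as BeginPlay, Tick and the construction script are empty.
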(event `self.ReceiveBeginPlay`)

(event `self.ReceiveTick`
  (params (DeltaSeconds :type "Float (single-precision)")))

(event `self.ReceiveAnyDamage`
  (params (Damage :type "Float (single-precision)") (DamageType :type "DamageType Object Reference") (InstigatedBy :type "Controller Object Reference") (DamageCauser :type "Actor Object Reference"))
  (`KismetSystemLibrary.PrintString` (`KismetStringLibrary.Conv_DoubleToString` Damage))
  (`PaperFlipbookComponent.SetFlipbook` (`self.Sprite`) "/Game/Assets/ImpactEffects/FB_BounceOrbDetonate.FB_BounceOrbDetonate")
  (`KismetSystemLibrary.Delay` 0.5)
  (`self.SetActorHiddenInGame` true)
  (`self.SetActorEnableCollision` false)
  (`PaperFlipbookComponent.SetFlipbook` (`self.Sprite`) "/Game/Assets/ImpactEffects/FP_BounceOrbIdle.FP_BounceOrbIdle")
  (`KismetSystemLibrary.Delay` 3.0)
  (`self.SetActorHiddenInGame` false)
  (`self.SetActorEnableCollision` true))

(fn `UserConstructionScript`)